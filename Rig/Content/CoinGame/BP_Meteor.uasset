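; BP_Meteor is a giant meteor that starts high in the air, falls and explodes on impact, knocking back nearby player characters.
; Each tick it aligns its Sphere to its velocity and shakes nearby cameras.
; On hit, DoBOOM pushes characters overlapping the Damage component away with a distance-attenuated impulse, alongside explosion effects and another shake.
; PushCharacter also adds damage to BP_PlayerState, though its distance terms cancel out.
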(event `self.ReceiveBeginPlay`
  (`self.SetActorScale3D` (30.0 30.0 30.0))
  (`self.K2_AddActorWorldOffset` (0.0 0.0 50000.0)))

(event `self.ReceiveTick`
  (params (DeltaSeconds :type "Float (single-precision)"))
  (bind _sphere (`self.Sphere`))
  (`SceneComponent.K2_SetWorldRotation` _sphere (`KismetMathLibrary.Conv_VectorToRotator` (`SceneComponent.GetComponentVelocity` _sphere)) false false)
  (`GameplayStatics.PlayWorldCameraShake` "/Game/CoinGame/BP_CameraShake.BP_CameraShake_C" (`SceneComponent.K2_GetComponentLocation` (`self.Sphere`)) 0.0 5000.0))

(event `self.Sphere.OnComponentHit`
  (params (HitComponent :type "PrimitiveComponent Object Reference") (OtherActor :type "Actor Object Reference") (OtherComp :type "PrimitiveComponent Object Reference") (NormalImpulse :type "Vector Structure") (Hit :type "HitResult Structure (by ref)"))
  (bind _returnvalue (`self.K2_GetActorLocation`))
  (`self.DoBOOM`)
  (`self.K2_DestroyActor`)
  (`GameplayStatics.SpawnEmitterAtLocation` "/Game/StarterContent/Particles/P_Explosion.P_Explosion" _returnvalue (`self.K2_GetActorRotation`) (100.0 100.0 100.0))
  (`GameplayStatics.PlayWorldCameraShake` "/Game/CoinGame/BP_CameraShake.BP_CameraShake_C" _returnvalue 0.0 5000.0))

(fn `AddRotation`
  (`SceneComponent.K2_AddLocalRotation` (`self.Sphere`) (struct :`Yaw` 1.0) false false))

(fn `DestroyActor`)

(fn `DoBOOM`
  (for _array_element (`PrimitiveComponent.GetOverlappingActors` (`self.Damage`) "/Game/aaaaa/ThirdPerson/Blueprints/BP_ThirdPersonCharacter.BP_ThirdPersonCharacter_C")
    (bind _asbp_third_person_character (cast `/Game/aaaaa/ThirdPerson/Blueprints/BP_ThirdPersonCharacter` _array_element))
    (`self.PushCharacter` _asbp_third_person_character))
  (`GameplayStatics.SpawnEmitterAtLocation` "/Game/StarterContent/Particles/P_Explosion.P_Explosion" (`self.K2_GetActorLocation`) (`self.K2_GetActorRotation`) (100.0 100.0 100.0))
  (`self.K2_DestroyActor`))

(fn `EventHitCharacter`
  (params (Actor :type "Actor Object Reference")))

(fn `Firework`
  (`NiagaraFunctionLibrary.SpawnSystemAtLocation` "/Game/CoinGame/Good.Good" (`SceneComponent.K2_GetComponentLocation` (`self.Sphere`)))
  (`self.K2_DestroyActor`))

(fn `PushCharacter`
  (params (Character :type "/Game/aaaaa/ThirdPerson/Blueprints/BP_ThirdPersonCharacter Object Reference"))
  (bind _returnvalue (`KismetMathLibrary.FClamp` (* (`KismetMathLibrary.Vector_Distance` (`self.K2_GetActorLocation` Character) (`self.K2_GetActorLocation`)) 0.01) 1.0 3.0))
  (bind _returnvalue_2 (/ (`self.MaxImpulse`) _returnvalue))
  (bind _asbp_player_state (cast `/Game/CoinGame/GameMode/BP_PlayerState` (`Pawn.PlayerState` Character)))
  (`/Game/CoinGame/GameMode/BP_PlayerState.AddDamage` _asbp_player_state (* _returnvalue (/ _returnvalue_2 500000.0)))
  (`CharacterMovementComponent.AddImpulse` (`Character.CharacterMovement` Character) (* (`KismetMathLibrary.GetForwardVector` (`KismetMathLibrary.FindLookAtRotation` (`self.K2_GetActorLocation`) (`self.K2_GetActorLocation` Character))) _returnvalue_2) false))

(fn `UserConstructionScript`)

(fn `VRotation`)