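; BP_TPArrow is a teleport arrow projectile that moves its owner to wherever it lands.
; On BeginPlay it gets a physics impulse scaled by Power along its forward vector with slight random spread, and Tick aligns it to its velocity until impact.
; Hit or overlap stops physics and collision, teleports the owner, spawns an effect, zeroes BP_ThirdPersonCharacter's Highest value via NOFALL, and destroys the arrow.
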(event `self.ReceiveTick`
  (params (DeltaSeconds :type "Float (single-precision)"))
  (if (`self.IsHit`)
    (`PrimitiveComponent.SetSimulatePhysics` (`self.SM_Arrow`) false)
    (else
      (`self.K2_SetActorRotation` (`KismetMathLibrary.Conv_VectorToRotator` (`SceneComponent.GetComponentVelocity` (`self.SM_Arrow`)))))))

(event `self.ReceiveBeginPlay`
  (`PrimitiveComponent.AddImpulse` (`self.SM_Arrow`) (* (`KismetMathLibrary.VLerp` (`KismetMathLibrary.RandomUnitVector`) (`self.GetActorForwardVector`) 0.95) (`self.Power`)) "None" false))

(event `self.SM_Arrow.OnComponentHit`
  (params (HitComponent :type "PrimitiveComponent Object Reference") (OtherActor :type "Actor Object Reference") (OtherComp :type "PrimitiveComponent Object Reference") (NormalImpulse :type "Vector Structure") (Hit :type "HitResult Structure (by ref)"))
  (set `self.IsHit` true)
  (`PrimitiveComponent.SetSimulatePhysics` (`self.SM_Arrow`) false)
  (`PrimitiveComponent.SetCollisionEnabled` (`self.SM_Arrow`) "NoCollision")
  (`self.NOFALL`)
  (`self.TPP`)
  (`self.K2_DestroyActor`))

(event `TPP`
  (bind _returnvalue (`self.K2_GetActorLocation`))
  (`self.K2_SetActorLocation` (`self.GetOwner`) _returnvalue false false)
  (`NiagaraFunctionLibrary.SpawnSystemAtLocation` null _returnvalue)
  (`self.K2_DestroyActor`))

(event `NOFALL`
  (bind _asbp_third_person_character (cast `/Game/ThirdPerson/Blueprints/BP_ThirdPersonCharacter` (`self.GetOwner`)))
  (set `/Game/ThirdPerson/Blueprints/BP_ThirdPersonCharacter.Highest` 0.0 _asbp_third_person_character))

(event `self.SM_Arrow.OnComponentBeginOverlap`
  (params (OverlappedComponent :type "PrimitiveComponent Object Reference") (OtherActor :type "Actor Object Reference") (OtherComp :type "PrimitiveComponent Object Reference") (OtherBodyIndex :type Integer) (bFromSweep :type Boolean) (SweepResult :type "HitResult Structure (by ref)"))
  (bind _returnvalue (`self.K2_GetActorLocation`))
  (`PrimitiveComponent.SetSimulatePhysics` (`self.SM_Arrow`) false)
  (`PrimitiveComponent.SetCollisionEnabled` (`self.SM_Arrow`) "NoCollision")
  (set `self.IsHit` true)
  (`self.K2_SetActorLocation` (`self.GetOwner`) _returnvalue false false)
  (`NiagaraFunctionLibrary.SpawnSystemAtLocation` null _returnvalue)
  (`self.NOFALL`)
  (`self.TPP`)
  (`self.K2_DestroyActor`))

(fn `UserConstructionScript`)