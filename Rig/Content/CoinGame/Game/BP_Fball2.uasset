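; BP_Fball2 is an explosive projectile, launched forward with slight random spread and removed after 15 seconds.
; Its physics sphere faces its velocity and, on any hit, explodes with sound, particles and camera shake, adding damage to player characters it strikes.
; A radial overlap on Sphere1 applies distance-scaled damage, ragdoll and knockback, but its collision is disabled on spawn and the re-enable node is unconnected.
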(event `self.ReceiveBeginPlay`
  (`PrimitiveComponent.SetCollisionEnabled` (`self.Sphere1`) "NoCollision")
  (`PrimitiveComponent.AddImpulse` (`self.Sphere`) (* (`KismetMathLibrary.VLerp` (`KismetMathLibrary.RandomUnitVector`) (`self.GetActorForwardVector`) 0.95) (`self.Power`)) "None" false)
  (`KismetSystemLibrary.Delay` 15.0)
  (`self.K2_DestroyActor`))

(event `self.ReceiveTick`
  (params (DeltaSeconds :type "Float (single-precision)"))
  (bind _sphere (`self.Sphere`))
  (`SceneComponent.K2_SetWorldRotation` _sphere (`KismetMathLibrary.Conv_VectorToRotator` (`SceneComponent.GetComponentVelocity` _sphere)) false false))

(event `self.Sphere.OnComponentHit`
  (params (HitComponent :type "PrimitiveComponent Object Reference") (OtherActor :type "Actor Object Reference") (OtherComp :type "PrimitiveComponent Object Reference") (NormalImpulse :type "Vector Structure") (Hit :type "HitResult Structure (by ref)"))
  (bind _asbp_third_person_character (cast `/Game/aaaaa/ThirdPerson/Blueprints/BP_ThirdPersonCharacter` OtherActor)
    (:`then`
      (bind _asbp_player_state (cast `/Game/CoinGame/GameMode/BP_PlayerState` (`Pawn.PlayerState` _asbp_third_person_character)))
      (`/Game/CoinGame/GameMode/BP_PlayerState.AddDamage` _asbp_player_state 1.0))
    (:`CastFailed`
      _))
  (`self.DestryBullet`))

(event `self.Sphere1.OnComponentBeginOverlap`
  (params (OverlappedComponent :type "PrimitiveComponent Object Reference") (OtherActor :type "Actor Object Reference") (OtherComp :type "PrimitiveComponent Object Reference") (OtherBodyIndex :type Integer) (bFromSweep :type Boolean) (SweepResult :type "HitResult Structure (by ref)"))
  (bind _returnvalue (`self.GetDistanceTo` OtherActor))
  (bind _sphereradius (`SphereComponent.SphereRadius` (`self.Sphere1`)))
  (bind _asbp_third_person_character (cast `/Game/aaaaa/ThirdPerson/Blueprints/BP_ThirdPersonCharacter` OtherActor))
  (bind _asbp_player_state (cast `/Game/CoinGame/GameMode/BP_PlayerState` (`Pawn.PlayerState` _asbp_third_person_character)))
  (`/Game/CoinGame/GameMode/BP_PlayerState.AddDamage` _asbp_player_state (/ (- _sphereradius _returnvalue) 5000.0))
  (`/Game/aaaaa/ThirdPerson/Blueprints/BP_ThirdPersonCharacter.DoRagdoll` _asbp_third_person_character)
  (`PrimitiveComponent.AddImpulse` (`Character.Mesh` _asbp_third_person_character) (* (* (`KismetMathLibrary.GetForwardVector` (`KismetMathLibrary.FindLookAtRotation` (`self.K2_GetActorLocation`) (`self.K2_GetActorLocation` _asbp_third_person_character))) (- _sphereradius _returnvalue)) 1.0) "None" false))

(fn `AddRotation`
  (`SceneComponent.K2_AddLocalRotation` (`self.Sphere`) (struct :`Yaw` 1.0) false false))

(fn `DestroyActor`)

(fn `DestryBullet`
  (bind _returnvalue (`self.K2_GetActorLocation`))
  (`GameplayStatics.SpawnSoundAtLocation` "/Game/StarterContent/Audio/Explosion_Cue.Explosion_Cue" (`self.K2_GetActorLocation`) (struct) 1.0 1.0 0.0 null null)
  (`self.K2_DestroyActor`)
  (`GameplayStatics.SpawnEmitterAtLocation` "/Game/StarterContent/Particles/P_Explosion.P_Explosion" _returnvalue (`self.K2_GetActorRotation`) (* (`self.GetActorScale3D`) 3.0))
  (`GameplayStatics.PlayWorldCameraShake` "/Game/CoinGame/BP_CameraShake.BP_CameraShake_C" _returnvalue 0.0 500.0))

(fn `EventHitCharacter`
  (params (Actor :type "Actor Object Reference")))

(fn `Firework`
  (`NiagaraFunctionLibrary.SpawnSystemAtLocation` "/Game/CoinGame/Good.Good" (`SceneComponent.K2_GetComponentLocation` (`self.Sphere`)))
  (`self.K2_DestroyActor`))

(fn `UserConstructionScript`)

(fn `VRotation`)