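; Player state for the coin game, holding HP, mana, shield, EXP, level, and coin and item counts.
; Damage drains shield before HP; damage and mana use pause regeneration, which resumes through a retriggerable delay and looping timer.
; EXP overflow levels up, rescaling stats and refilling HP and mana.
; Stat changes broadcast through an event dispatcher, while most counters update BP_Hud directly, except AddBlack, which uses its own dispatcher.
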(event `self.ReceiveBeginPlay`
  (bind _structout (setmembers `/Game/CoinGame/GameMode/ST_PlayerState` :`StructRef` (`self.PlayerState`) :`CurHP` 100.0 :`MaxHp` 100.0 :`CurShield` 100.0 :`MaxShield` 100.0 :`Mana` 0.0 :`MaxMana` 10.0 :`Exp` 0 :`MaxExp` 100 :`Level` 0 :`MaxLevel` 1000 :`Damage` 1.0))
  (`self.EventDispatcher_Change` _structout)
  (`self.재생HP`)
  (`self.재생Mana`))

(event `재생Mana`
  (`KismetSystemLibrary.RetriggerableDelay` 1.0)
  (bind _returnvalue (`KismetSystemLibrary.K2_SetTimerDelegate` (delegate `재생ManaON`) (`self.Delta Seconds`) true))
  (set `self.Mana재생` _returnvalue))

(event `재생ManaON`
  (bind (_playerstate_curhp _playerstate_maxhp _playerstate_curshield _playerstate_maxshield _playerstate_mana _playerstate_maxmana) (break `/Game/CoinGame/GameMode/ST_PlayerState` (`self.PlayerState`)))
  (bind _playerstate (`self.PlayerState`))
  (if (< _playerstate_mana _playerstate_maxmana)
    (setmembers `/Game/CoinGame/GameMode/ST_PlayerState` :`StructRef` _playerstate :`Mana` (+ _playerstate_mana (`self.Delta Seconds`)))
    (`self.EventDispatcher_Change` _playerstate)))

(event `UseMana`
  (params (`MANA-` :type "Float (double-precision)"))
  (bind _playerstate (`self.PlayerState`))
  (bind ((`Mana_15_A922942F459E481374D563A429A598C1` _mana) (`MaxMana_14_380C5C9E416070CBFA88B4BA18E6090B` _maxmana)) (break `/Game/CoinGame/GameMode/ST_PlayerState` (`self.PlayerState`)))
  (`KismetSystemLibrary.K2_ClearAndInvalidateTimerHandle` (`self.Mana재생`))
  (setmembers `/Game/CoinGame/GameMode/ST_PlayerState` :`StructRef` _playerstate :`Mana` (`KismetMathLibrary.FClamp` (- _mana (* (`self.Delta Seconds`) 5.0) `MANA-`) 0.0 _maxmana))
  (`self.EventDispatcher_Change` _playerstate)
  (`self.재생Mana`))

(event `self.ReceiveTick`
  (params (DeltaSeconds :type "Float (single-precision)"))
  (set `self.Delta Seconds` DeltaSeconds))

(event `재생HP`
  (`KismetSystemLibrary.RetriggerableDelay` 1.0)
  (bind _returnvalue (`KismetSystemLibrary.K2_SetTimerDelegate` (delegate `재생HPON`) (`self.Delta Seconds`) true))
  (set `self.HP재생` _returnvalue))

(event `재생HPON`
  (bind (_playerstate_curhp _playerstate_maxhp) (break `/Game/CoinGame/GameMode/ST_PlayerState` (`self.PlayerState`)))
  (bind _playerstate (`self.PlayerState`))
  (if (< _playerstate_curhp _playerstate_maxhp)
    (setmembers `/Game/CoinGame/GameMode/ST_PlayerState` :`StructRef` _playerstate :`CurHP` (+ _playerstate_curhp (* (`self.Delta Seconds`) 2.0)))
    (`self.EventDispatcher_Change` _playerstate)))

(fn `AddBlack`
  (bind _output_get (set `self.BlackItem` (+ (`self.BlackItem`) 1)))
  (`self.EventDispatcher_ChangeBlackItem` _output_get))

(fn `AddBlackItem`
  (bind _output_get (set `self.BlackItem` (+ (`self.BlackItem`) 1)))
  (bind _asbp_hud (cast `/Game/CoinGame/GameMode/BP_Hud` (`PlayerController.GetHUD` (`GameplayStatics.GetPlayerController` 0))))
  (`/Game/CoinGame/GameMode/BP_Hud.SetBlackItemText` _asbp_hud _output_get))

(fn `AddCoin`
  (bind _output_get (set `self.Coin` (+ (`self.Coin`) 1)))
  (bind _asbp_hud (cast `/Game/CoinGame/GameMode/BP_Hud` (`PlayerController.GetHUD` (`GameplayStatics.GetPlayerController` 0))))
  (`/Game/CoinGame/GameMode/BP_Hud.SetCoinText` _asbp_hud _output_get))

(fn `AddDamage`
  (params (Damage :type "Float (double-precision)"))
  (bind (_playerstate_curhp _playerstate_maxhp) (break `/Game/CoinGame/GameMode/ST_PlayerState` (`self.PlayerState`)))
  (bind _playerstate (`self.PlayerState`))
  (`KismetSystemLibrary.K2_ClearAndInvalidateTimerHandle` (`self.HP재생`))
  (bind _remaindamage (`self.AddShieldDamage` Damage))
  (if (> _playerstate_curhp 0.0)
    (setmembers `/Game/CoinGame/GameMode/ST_PlayerState` :`StructRef` _playerstate :`CurHP` (`KismetMathLibrary.FClamp` (- _playerstate_curhp _remaindamage) 0.0 _playerstate_maxhp))
    (`self.EventDispatcher_Change` _playerstate)
    (`self.재생HP`)))

(fn `AddEXP`
  (params (EXP :type Integer))
  (bind _playerstate (`self.PlayerState`))
  (bind (_playerstate_curhp _playerstate_maxhp _playerstate_curshield _playerstate_maxshield _playerstate_mana _playerstate_maxmana _playerstate_exp _playerstate_maxexp _playerstate_level) (break `/Game/CoinGame/GameMode/ST_PlayerState` (`self.PlayerState`)))
  (bind _playerstate_2 (`self.PlayerState`))
  (bind (_playerstate_curhp_2 _playerstate_maxhp_2 _playerstate_curshield_2 _playerstate_maxshield_2 _playerstate_mana_2 _playerstate_maxmana_2 _playerstate_exp_2 _playerstate_maxexp_2) (break `/Game/CoinGame/GameMode/ST_PlayerState` (`self.PlayerState`)))
  (bind _returnvalue (+ _playerstate_exp_2 EXP))
  (bind _returnvalue_2 (/ _playerstate_level 5))
  (bind _returnvalue_3 (`KismetMathLibrary.Conv_IntToDouble` (+ (* _playerstate_level 10) 100)))
  (if (>= _returnvalue _playerstate_maxexp_2)
    (setmembers `/Game/CoinGame/GameMode/ST_PlayerState` :`StructRef` _playerstate :`Exp` (- _returnvalue _playerstate_maxexp) :`Level` (+ _playerstate_level 1))
    (setmembers `/Game/CoinGame/GameMode/ST_PlayerState` :`StructRef` _playerstate :`CurHP` _returnvalue_3 :`MaxHp` _returnvalue_3 :`Mana` _playerstate_maxmana :`MaxMana` (`KismetMathLibrary.Conv_IntToDouble` (+ (* _playerstate_level 10) 10)) :`MaxExp` (+ (+ (* _playerstate_level 100) (* _returnvalue_2 100)) 100) :`Damage` (`KismetMathLibrary.Conv_IntToDouble` (+ (* _playerstate_level 3) (* _returnvalue_2 10))))
    (`self.EventDispatcher_Change` _playerstate)
    (else
      (setmembers `/Game/CoinGame/GameMode/ST_PlayerState` :`StructRef` _playerstate_2 :`Exp` (`KismetMathLibrary.Clamp` _returnvalue 0 _playerstate_maxexp_2))
      (`self.EventDispatcher_Change` _playerstate_2))))

(fn `AddGreenItem`
  (bind _output_get (set `self.GreenItem` (+ (`self.GreenItem`) 1)))
  (bind _asbp_hud (cast `/Game/CoinGame/GameMode/BP_Hud` (`PlayerController.GetHUD` (`GameplayStatics.GetPlayerController` 0))))
  (`/Game/CoinGame/GameMode/BP_Hud.SetGreenItemText` _asbp_hud _output_get))

(fn `AddHeal`
  (params (Heal :type "Float (double-precision)"))
  (bind _playerstate (`self.PlayerState`))
  (bind (_playerstate_curhp _playerstate_maxhp) (break `/Game/CoinGame/GameMode/ST_PlayerState` (`self.PlayerState`)))
  (if (< _playerstate_curhp _playerstate_maxhp)
    (setmembers `/Game/CoinGame/GameMode/ST_PlayerState` :`StructRef` _playerstate :`CurHP` (`KismetMathLibrary.FClamp` (+ _playerstate_curhp Heal) 0.0 _playerstate_maxhp))
    (`self.EventDispatcher_Change` _playerstate)))

(fn `AddRedItem`
  (bind _output_get (set `self.RedItem` (+ (`self.RedItem`) 1)))
  (bind _asbp_hud (cast `/Game/CoinGame/GameMode/BP_Hud` (`PlayerController.GetHUD` (`GameplayStatics.GetPlayerController` 0))))
  (`/Game/CoinGame/GameMode/BP_Hud.SetRedItemText` _asbp_hud _output_get))

(fn `AddShieldDamage`
  (params (Damage :type "Float (double-precision)"))
  (returns (RemainDamage :type "Float (double-precision)"))
  (bind (_playerstate_curhp _playerstate_maxhp _playerstate_curshield) (break `/Game/CoinGame/GameMode/ST_PlayerState` (`self.PlayerState`)))
  (bind _playerstate (`self.PlayerState`))
  (bind _returnvalue (- _playerstate_curshield Damage))
  (if (> _returnvalue 0.0)
    (setmembers `/Game/CoinGame/GameMode/ST_PlayerState` :`StructRef` _playerstate :`CurShield` _returnvalue)
    (return 0.0)
    (else
      (setmembers `/Game/CoinGame/GameMode/ST_PlayerState` :`StructRef` _playerstate :`CurShield` 0.0)
      (return (`KismetMathLibrary.Abs` _returnvalue)))))

(fn `AddShieldHeal`
  (params (AddShieldHeal :type "Float (double-precision)"))
  (bind _playerstate (`self.PlayerState`))
  (bind (_playerstate_curhp _playerstate_maxhp _playerstate_curshield _playerstate_maxshield) (break `/Game/CoinGame/GameMode/ST_PlayerState` (`self.PlayerState`)))
  (if (< _playerstate_curshield _playerstate_maxshield)
    (setmembers `/Game/CoinGame/GameMode/ST_PlayerState` :`StructRef` _playerstate :`CurShield` (`KismetMathLibrary.FClamp` (+ _playerstate_curshield AddShieldHeal) 0.0 _playerstate_maxshield))
    (`self.EventDispatcher_Change` _playerstate)))

(fn `Ragdoll`)

(fn `UseBlackItem`
  (bind _output_get (set `self.BlackItem` (+ (`self.BlackItem`) -1)))
  (bind _asbp_hud (cast `/Game/CoinGame/GameMode/BP_Hud` (`PlayerController.GetHUD` (`GameplayStatics.GetPlayerController` 0))))
  (`/Game/CoinGame/GameMode/BP_Hud.SetBlackItemText` _asbp_hud _output_get))

(fn `UseGreenItem`
  (bind _output_get (set `self.GreenItem` (+ (`self.GreenItem`) -1)))
  (bind _asbp_hud (cast `/Game/CoinGame/GameMode/BP_Hud` (`PlayerController.GetHUD` (`GameplayStatics.GetPlayerController` 0))))
  (`/Game/CoinGame/GameMode/BP_Hud.SetGreenItemText` _asbp_hud _output_get))

(fn `UserConstructionScript`)

(fn `UseRedItem`
  (bind _output_get (set `self.RedItem` (+ (`self.RedItem`) -1)))
  (bind _asbp_hud (cast `/Game/CoinGame/GameMode/BP_Hud` (`PlayerController.GetHUD` (`GameplayStatics.GetPlayerController` 0))))
  (`/Game/CoinGame/GameMode/BP_Hud.SetRedItemText` _asbp_hud _output_get))