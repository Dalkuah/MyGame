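; AI spawner that places random entities from a configurable set inside a box sized by SpawnRadius.
; It binds to game state changes, with Play starting a looping spawn timer and Ready clearing it.
; Each wave line-traces downward for spawn locations, then passes HP and damage scaled by accumulated time.
; Tick randomizes delay and rate, accumulates time below the population cap, stops spawning above it and prunes invalid actors.
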(event `self.ReceiveBeginPlay`
  (`self.BindGameState`)
  (`KismetSystemLibrary.K2_SetTimer` null "Spawn" 0.0 true))

(event `self.ReceiveTick`
  (params (DeltaSeconds :type "Float (single-precision)"))
  (bind _spawnmaxdelay (`self.SpawnMaxDelay`))
  (bind _spawnmaxrate (`self.SpawnMaxRate`))
  (bind _spawncount (`self.SpawnCount`))
  (`|ExecutionSequence`
    (:`then_0`
      (if (<= (`KismetArrayLibrary.Array_Length` (`self.SpawnCount`)) (`self.MaxAmount`))
        (`KismetSystemLibrary.K2_SetTimer` null "Spawn")
        (`BoxComponent.SetBoxExtent` (`self.Bound`) (`KismetMathLibrary.Conv_DoubleToVector` (`self.SpawnRadius`)) true)
        (set `self.TotalSec` (+ (`self.TotalSec`) DeltaSeconds))
        (`|ExecutionSequence`
          (:`then_0`
            (if (== (`self.SpawnMaxDelay`) 0.0)
              (set `self.SpawnDelay` 10.0)
              (else
                (set `self.SpawnDelay` (`KismetMathLibrary.FClamp` (`KismetMathLibrary.RandomFloatInRange` (`self.SpawnMinDelay`) _spawnmaxdelay) 0.0 _spawnmaxdelay)))))
          (:`then_1`
            (if (== (`self.SpawnMaxRate`) 0)
              (set `self.SpawnRate` 3)
              (else
                (set `self.SpawnRate` (`KismetMathLibrary.Clamp` (`KismetMathLibrary.RandomIntegerInRange` (`self.SpawnMinRate`) _spawnmaxrate) 0 _spawnmaxrate)))))
          (:`then_2`
            (if (== (`self.MaxAmount`) 0)
              (set `self.MaxAmount` 3))))
        (else
          (`KismetSystemLibrary.K2_ClearTimer` null "Spawn2"))))
    (:`then_1`
      (for (_array_element _array_index) _spawncount
        (`/Engine/EditorBlueprintResources/StandardMacros.IsValid` _array_element
          (:`Is Not Valid`
            (`KismetArrayLibrary.Array_Remove` _spawncount _array_index)))))))

(fn `BindGameState`
  (bind _asbp_game_state (cast `/Game/CoinGame/GameMode/BP_GameState` (`GameplayStatics.GetGameState`)))
  (add `/Game/CoinGame/GameMode/BP_GameState.EventDispatcher_ChangeGameState` _asbp_game_state (`|CreateDelegate` :!event `Spawn`)))

(fn `Spawn`
  (params (Game :type "/Game/CoinGame/GameMode/EN_GameState Enum" :default "NewEnumerator4"))
  (switch `/Game/CoinGame/GameMode/EN_GameState` Game
    (:`NewEnumerator0`
      (`KismetSystemLibrary.K2_ClearTimer` null "Spawn2"))
    (:`NewEnumerator1`
      (`self.Spawn2`)
      (`KismetSystemLibrary.K2_SetTimer` null "Spawn2" (`self.SpawnDelay`) true))))

(fn `Spawn2`
  (bind (_origin _boxextent) (`KismetSystemLibrary.GetComponentBounds` (`self.Bound`)))
  (bind _returnvalue (/ (`self.TotalSec`) 5.0))
  (bind _returnvalue_2 (`KismetMathLibrary.MakeVector` (.x (`KismetMathLibrary.RandomPointInBoundingBox` _origin _boxextent)) (.y (`KismetMathLibrary.RandomPointInBoundingBox` _origin _boxextent)) (+ (.z (`KismetMathLibrary.RandomPointInBoundingBox` _origin _boxextent)) 10000.0)))
  (for _ (range 1 (+ (`self.SpawnRate`) 1))
    (bind _outhit (`KismetSystemLibrary.LineTraceSingleForObjects` _returnvalue_2 (+ _returnvalue_2 (* (* (`self.GetActorUpVector`) -1) 15000.0)) (`|MakeArray` "ObjectTypeQuery1" :!type "EObjectTypeQuery Enum")))
    (bind _returnvalue_3 (`|SpawnActorFromClass` (`KismetArrayLibrary.Array_Random` (`self.SetEntity`)) (`KismetMathLibrary.MakeTransform` (`.ImpactPoint` (`GameplayStatics.BreakHitResult` _outhit)) (`KismetMathLibrary.MakeRotator` 0.0 0.0 (`KismetMathLibrary.RandomFloat`))) "Undefined" "OverrideRootScale" null null))
    (`KismetArrayLibrary.Array_Add` (`self.SpawnCount`) _returnvalue_3)
    (`/Engine/EditorBlueprintResources/StandardMacros.IsValid` _returnvalue_3
      (:`Is Valid`
        (message `/Game/CoinGame/AISet.AISET` _returnvalue_3 _returnvalue (/ _returnvalue 3.0))))))

(fn `UserConstructionScript`)