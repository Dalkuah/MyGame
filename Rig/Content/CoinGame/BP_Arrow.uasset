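; BP_Arrow is a physics-driven arrow projectile that damages player characters and AI.
; On spawn it gets a forward impulse scaled by Power with slight random spread, then orients along its velocity in flight.
; Hits stop it, while overlaps also attach it to the touched component, apply damage through BP_PlayerState or BP_AI and spawn blood FX.
; A Delay started from Tick during flight destroys it after five seconds.
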(event `self.ReceiveTick`
  (params (DeltaSeconds :type "Float (single-precision)"))
  (if (`self.IsHit`)
    (`PrimitiveComponent.SetSimulatePhysics` (`self.SM_Arrow`) false)
    (else
      (`self.K2_SetActorRotation` (`KismetMathLibrary.Conv_VectorToRotator` (`SceneComponent.GetComponentVelocity` (`self.SM_Arrow`))))
      (`KismetSystemLibrary.Delay` 5.0)
      (`self.K2_DestroyActor`))))

(event `self.ReceiveBeginPlay`
  (`PrimitiveComponent.AddImpulse` (`self.SM_Arrow`) (* (`KismetMathLibrary.VLerp` (`KismetMathLibrary.RandomUnitVector`) (`self.GetActorForwardVector`) 0.95) (`self.Power`)) "None" false))

(event `self.SM_Arrow.OnComponentHit`
  (params (HitComponent :type "PrimitiveComponent Object Reference") (OtherActor :type "Actor Object Reference") (OtherComp :type "PrimitiveComponent Object Reference") (NormalImpulse :type "Vector Structure") (Hit :type "HitResult Structure (by ref)"))
  (set `self.IsHit` true)
  (`PrimitiveComponent.SetSimulatePhysics` (`self.SM_Arrow`) false)
  (`PrimitiveComponent.SetCollisionEnabled` (`self.SM_Arrow`) "NoCollision"))

(event `self.SM_Arrow.OnComponentBeginOverlap`
  (params (OverlappedComponent :type "PrimitiveComponent Object Reference") (OtherActor :type "Actor Object Reference") (OtherComp :type "PrimitiveComponent Object Reference") (OtherBodyIndex :type Integer) (bFromSweep :type Boolean) (SweepResult :type "HitResult Structure (by ref)"))
  (bind _returnvalue (`self.GetTransform`))
  (`PrimitiveComponent.SetSimulatePhysics` (`self.SM_Arrow`) false)
  (`PrimitiveComponent.SetCollisionEnabled` (`self.SM_Arrow`) "NoCollision")
  (`self.K2_AttachToComponent` OtherComp "None" "KeepWorld" "KeepWorld" "KeepRelative")
  (if (not (`self.IsHit`))
    (`|ExecutionSequence`
      (:`then_0`
        (bind _asbp_third_person_character (cast `/Game/aaaaa/ThirdPerson/Blueprints/BP_ThirdPersonCharacter` OtherActor))
        (bind _asbp_player_state (cast `/Game/CoinGame/GameMode/BP_PlayerState` (`Pawn.PlayerState` _asbp_third_person_character)))
        (`/Game/CoinGame/GameMode/BP_PlayerState.AddDamage` _asbp_player_state 10.0))
      (:`then_1`
        (bind _asbp_ai (cast `/Game/MyGame/AI/BP_AI` OtherActor))
        (`/Game/MyGame/AI/BP_AI.AddDamage` _asbp_ai 10.0)))
    (`NiagaraFunctionLibrary.SpawnSystemAtLocation` "/Game/CoinGame/BloodFx.BloodFx" (.location _returnvalue) (`KismetMathLibrary.MakeRotator` (.roll (.rotation _returnvalue)) (.pitch (.rotation _returnvalue)) (.yaw (.rotation _returnvalue))) (.scale _returnvalue))
    (set `self.IsHit` true)))

(fn `UserConstructionScript`)