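; BP_Homing is a homing projectile in the coin game that chases the first player character.
; Tick moves it along its Arrow's forward vector while interpolating its rotation toward the target.
; Any sphere overlap explodes it with a camera shake, first adding damage to BP_PlayerState and knocking back the character if it is a BP_ThirdPersonCharacter.
; Without a hit, a BeginPlay delay ends it with a Niagara effect.
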(event `self.ReceiveTick`
  (params (DeltaSeconds :type "Float (single-precision)"))
  (`/Engine/EditorBlueprintResources/StandardMacros.IsValid` (`self.HomingTarget`)
    (:`Is Valid`
      (`self.K2_AddActorWorldOffset` (* (`SceneComponent.GetForwardVector` (`self.Arrow`)) (* DeltaSeconds 10000.0)))
      (`self.K2_SetActorRotation` (`KismetMathLibrary.RInterpTo` (`self.K2_GetActorRotation`) (`KismetMathLibrary.FindLookAtRotation` (`self.K2_GetActorLocation`) (`self.K2_GetActorLocation` (`self.HomingTarget`))) DeltaSeconds 5.0)))))

(event `TimeOver`
  (`NiagaraFunctionLibrary.SpawnSystemAtLocation` "/Game/CoinGame/Good.Good" (`self.K2_GetActorLocation`))
  (`ActorComponent.SetActive` (`self.DeathFx`) true false)
  (`self.K2_DestroyActor`))

(event `self.ReceiveBeginPlay`
  (set `self.HomingTarget` (`GameplayStatics.GetPlayerCharacter` 0))
  (`KismetSystemLibrary.Delay` 10.0)
  (`self.TimeOver`))

(event `self.Sphere.OnComponentBeginOverlap`
  (params (OverlappedComponent :type "PrimitiveComponent Object Reference") (OtherActor :type "Actor Object Reference") (OtherComp :type "PrimitiveComponent Object Reference") (OtherBodyIndex :type Integer) (bFromSweep :type Boolean) (SweepResult :type "HitResult Structure (by ref)"))
  (`self.EventHitCharacter` OtherActor)
  (`self.DestroyHoming`))

(fn `DestroyHoming`
  (bind _returnvalue (`self.K2_GetActorLocation`))
  (`GameplayStatics.SpawnEmitterAtLocation` "/Game/StarterContent/Particles/P_Explosion.P_Explosion" _returnvalue (`self.K2_GetActorRotation`))
  (`self.K2_DestroyActor`)
  (`GameplayStatics.PlayWorldCameraShake` "/Game/CoinGame/BP_CameraShake.BP_CameraShake_C" _returnvalue 0.0 500.0))

(fn `EventHitCharacter`
  (params (Actor :type "Actor Object Reference"))
  (bind _asbp_third_person_character (cast `/Game/aaaaa/ThirdPerson/Blueprints/BP_ThirdPersonCharacter` Actor))
  (bind _asbp_player_state (cast `/Game/CoinGame/GameMode/BP_PlayerState` (`Pawn.PlayerState` _asbp_third_person_character)))
  (`/Game/CoinGame/GameMode/BP_PlayerState.AddDamage` _asbp_player_state 7.0)
  (`CharacterMovementComponent.AddImpulse` (`Character.CharacterMovement` _asbp_third_person_character) (* (`SceneComponent.GetForwardVector` (`self.Arrow`)) 50000.0) false))

(fn `UserConstructionScript`)