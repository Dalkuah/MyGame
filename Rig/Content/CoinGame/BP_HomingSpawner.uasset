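; BP_HomingSpawner is a coin-game spawner that periodically creates BP_Homing actors from its Cube's transform, each with randomized rotation offsets.
; BeginPlay binds to the BP_GameState ChangeGameState dispatcher and also sets a looping timer on Spawn, which takes a game-state argument.
; Spawn clears the Spawn2 timer on Ready and starts it looping at SpawnDelay on Play.
; Each Spawn2 tick creates SpawnRate homing actors.
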(event `self.ReceiveBeginPlay`
  (`self.BindGameState`)
  (`KismetSystemLibrary.K2_SetTimer` null "Spawn" (`self.SpawnDelay`) true))

(fn `BindGameState`
  (bind _asbp_game_state (cast `/Game/CoinGame/GameMode/BP_GameState` (`GameplayStatics.GetGameState`)))
  (add `/Game/CoinGame/GameMode/BP_GameState.EventDispatcher_ChangeGameState` _asbp_game_state (`|CreateDelegate` :!event `Spawn`)))

(fn `Spawn`
  (params (Game :type "/Game/CoinGame/GameMode/EN_GameState Enum" :default "NewEnumerator4"))
  (switch `/Game/CoinGame/GameMode/EN_GameState` Game
    (:`NewEnumerator0`
      (`KismetSystemLibrary.K2_ClearTimer` null "Spawn2"))
    (:`NewEnumerator1`
      (`KismetSystemLibrary.K2_SetTimer` null "Spawn2" (`self.SpawnDelay`) true))))

(fn `Spawn2`
  (bind _returnvalue (`SceneComponent.K2_GetComponentToWorld` (`self.Cube`)))
  (for _ (range 1 (+ (`self.SpawnRate`) 1))
    (`|SpawnActorFromClass` "/Game/CoinGame/BP_Homing.BP_Homing_C" (`KismetMathLibrary.MakeTransform` (.location _returnvalue) (`KismetMathLibrary.MakeRotator` (+ (.roll (.rotation _returnvalue)) (`KismetMathLibrary.RandomFloatInRange` 0.0 360.0)) (+ (.pitch (.rotation _returnvalue)) (`KismetMathLibrary.RandomFloatInRange` 0.0 360.0)) (+ (.yaw (.rotation _returnvalue)) (`KismetMathLibrary.RandomFloatInRange` 0.0 360.0))) (.scale _returnvalue)) "Undefined" "OverrideRootScale" null null)))

(fn `UserConstructionScript`)