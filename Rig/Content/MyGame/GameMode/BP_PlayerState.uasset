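; BP_PlayerState holds a player stats struct and provides functions to apply damage and healing to HP.
; AddDamage runs only while HP is above zero, and AddHeal only while HP is below MaxHP.
; Both clamp the new HP between zero and MaxHP, then broadcast the updated struct through the Change event dispatcher.
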(fn `AddDamage`
  (params (Damage :type Integer))
  (bind (_all_hp _all_maxhp) (break `/Game/MyGame/ST_ALL` (`self.All`)))
  (bind _all (`self.All`))
  (if (> _all_hp 0)
    (setmembers `/Game/MyGame/ST_ALL` :`StructRef` _all :`HP` (`KismetMathLibrary.Clamp` (- _all_hp Damage) 0 _all_maxhp))
    (`self.EventDispatcherChange` _all)))

(fn `AddHeal`
  (params (Heal :type Integer))
  (bind (_all_hp _all_maxhp) (break `/Game/MyGame/ST_ALL` (`self.All`)))
  (bind _all (`self.All`))
  (if (< _all_hp _all_maxhp)
    (setmembers `/Game/MyGame/ST_ALL` :`StructRef` _all :`HP` (`KismetMathLibrary.Clamp` (+ _all_hp Heal) 0 _all_maxhp))
    (`self.EventDispatcherChange` _all)))

(fn `UserConstructionScript`)