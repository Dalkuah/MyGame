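; Hookshot actor attached to a camera-equipped owner that fires a chained hook along a camera line trace and reports state changes through a dispatcher.
; A state machine sends the hook to the trace point, then either holds it on a hit or retracts it faster on a miss.
; Tick stretches the chain using instanced links plus a scaled first link for the remainder, and interpolates camera FOV while in use or idle.
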(event `self.ReceiveBeginPlay`
  (`self.HandleSetHookShotState` "NewEnumerator1")
  (set `self.DefaultFieldOfView` (`CameraComponent.FieldOfView` (`self.GetComponentByClass` (`ActorComponent.GetOwner` (`SceneComponent.GetAttachParent` (`self.DefaultSceneRoot`))) "/Script/Engine.CameraComponent"))))

(event `self.ReceiveTick`
  (params (DeltaSeconds :type "Float (single-precision)"))
  (bind _currenthooklocation (`self.CurrentHookLocation`))
  (bind _returnvalue (`KismetMathLibrary.GetDirectionUnitVector` (`self.K2_GetActorLocation`) (`self.CurrentHookLocation`)))
  (bind _returnvalue_2 (`InstancedStaticMeshComponent.GetInstanceCount` (`self.InstancedChains`)))
  (bind (_remainder _returnvalue_3) (`KismetMathLibrary.FMod` (`KismetMathLibrary.Vector_Distance` (`self.K2_GetActorLocation`) (`self.CurrentHookLocation`)) (`self.ChainMeshLength`)))
  (bind _returnvalue_4 (`self.GetComponentByClass` (`ActorComponent.GetOwner` (`SceneComponent.GetAttachParent` (`self.DefaultSceneRoot`))) "/Script/Engine.CameraComponent"))
  (bind _returnvalue_5 (`self.GetComponentByClass` (`ActorComponent.GetOwner` (`SceneComponent.GetAttachParent` (`self.DefaultSceneRoot`))) "/Script/Engine.CameraComponent"))
  (`|ExecutionSequence`
    (:`then_0`
      (if (`|EnumInequality` (`self.HookShotState`) "NewEnumerator1")
        (`|ExecutionSequence`
          (:`then_0`
            ;[1 1 1] 코멘트
            (`SceneComponent.K2_SetWorldLocationAndRotation` (`self.Sphere`) _currenthooklocation (`KismetMathLibrary.Conv_VectorToRotator` (`KismetMathLibrary.GetDirectionUnitVector` (`self.K2_GetActorLocation`) _currenthooklocation)) false false))
          (:`then_1`
            ;[1 1 1] 코멘트
            (`SceneComponent.K2_SetWorldRotation` (`self.FirstChain`) (`KismetMathLibrary.Conv_VectorToRotator` (`KismetMathLibrary.GetDirectionUnitVector` (`self.K2_GetActorLocation`) (`self.CurrentHookLocation`))) false false)
            (`SceneComponent.SetRelativeScale3D` (`self.FirstChain`) (`KismetMathLibrary.MakeVector` (/ (`KismetMathLibrary.FMod` (`KismetMathLibrary.Vector_Distance` (`self.K2_GetActorLocation`) (`self.CurrentHookLocation`)) (`self.ChainMeshLength`)) (`self.ChainMeshLength`)) 1.0 1.0)))
          (:`then_2`
            ;[1 1 1] 코멘트
            (`SceneComponent.K2_SetWorldLocationAndRotation` (`self.InstancedChains`) (+ (`self.K2_GetActorLocation`) (* _returnvalue (`KismetMathLibrary.FMod` (`KismetMathLibrary.Vector_Distance` (`self.K2_GetActorLocation`) (`self.CurrentHookLocation`)) (`self.ChainMeshLength`)))) (`KismetMathLibrary.Conv_VectorToRotator` _returnvalue) false false)
            (if (> _returnvalue_3 _returnvalue_2)
              (for _index (range _returnvalue_2 _returnvalue_3)
                (`InstancedStaticMeshComponent.AddInstance` (`self.InstancedChains`) (`KismetMathLibrary.MakeTransform` (`KismetMathLibrary.MakeVector` (* _index (`self.ChainMeshLength`)))) false))
              (elif (< _returnvalue_3 _returnvalue_2)
                (for _index_2 (range _returnvalue_3 _returnvalue_2)
                  (`InstancedStaticMeshComponent.RemoveInstance` (`self.InstancedChains`) _index_2))))))))
    (:`then_1`
      (switch `/Game/MyGame/Hook/EN_HookShotState` (`self.HookShotState`)
        (:`NewEnumerator1`
          (`CameraComponent.SetFieldOfView` _returnvalue_4 (`KismetMathLibrary.FInterpTo` (`CameraComponent.FieldOfView` _returnvalue_4) (`self.DefaultFieldOfView`) DeltaSeconds 10.0)))
        (:`NewEnumerator2`
          (set `self.CurrentHookLocation` (`KismetMathLibrary.VInterpTo_Constant` (`self.CurrentHookLocation`) (`self.TargetHookShotLocation`) DeltaSeconds (`self.ChainSpeed`)))
          (if (== (`self.CurrentHookLocation`) (`self.TargetHookShotLocation`))
            (if (`self.HitSuccessful`)
              (`self.HandleSetHookShotState` "NewEnumerator4")
              (else
                (`self.HandleSetHookShotState` "NewEnumerator3")))))
        (:`NewEnumerator3`
          (set `self.CurrentHookLocation` (`KismetMathLibrary.VInterpTo_Constant` (`self.CurrentHookLocation`) (`self.K2_GetActorLocation`) DeltaSeconds (* (`self.ChainSpeed`) 2.5)))
          (if (== (`self.CurrentHookLocation`) (`self.K2_GetActorLocation`))
            (`self.HandleSetHookShotState` "NewEnumerator1")))
        (:`NewEnumerator4`
          (`CameraComponent.SetFieldOfView` _returnvalue_5 (`KismetMathLibrary.FInterpTo` (`CameraComponent.FieldOfView` _returnvalue_5) (`self.TargetInFieldOfView`) DeltaSeconds 6.0)))))))

(fn `CalculateHookShotHit`
  (params (CharacterCamera :type "CameraComponent Object Reference") (Character :type "Actor Object Reference"))
  (returns (EndCharacterLcoation :type "Vector Structure") (HitSuccessful :type Boolean))
  (bind _returnvalue (`SceneComponent.K2_GetComponentLocation` CharacterCamera))
  (bind (_outhit _returnvalue_2) (`KismetSystemLibrary.LineTraceSingle` _returnvalue (+ _returnvalue (* (`SceneComponent.GetForwardVector` CharacterCamera) (`self.HookShotRange`))) "TraceTypeQuery1" false (`|MakeArray` Character)))
  (if _returnvalue_2
    (bind (_bblockinghit _binitialoverlap _time _distance _location _impactpoint _normal _impactnormal _physmat _hitactor _hitcomponent _hitbonename _bonename _hititem _elementindex _faceindex _tracestart _traceend) (`GameplayStatics.BreakHitResult` _outhit))
    (set `self.TargetHookShotLocation` _impactpoint)
    (`self.HandleSetHookShotState` "NewEnumerator2")
    (set `self.HitSuccessful` true)
    (return _impactpoint true)
    (else
      (set `self.TargetHookShotLocation` _traceend)
      (`self.HandleSetHookShotState` "NewEnumerator2")
      (set `self.HitSuccessful` false)
      (return (0.0 0.0 0.0) (`self.HitSuccessful`)))))

(fn `HandleSetHookShotState`
  (params (NewHookShotState :type "/Game/MyGame/Hook/EN_HookShotState Enum" :default "NewEnumerator0"))
  (bind _output_get (set `self.HookShotState` NewHookShotState))
  (`self.OnHookShotStateChanged` _output_get)
  (switch `/Game/MyGame/Hook/EN_HookShotState` _output_get
    (:`NewEnumerator1`
      (`InstancedStaticMeshComponent.ClearInstances` (`self.InstancedChains`))
      (`SceneComponent.SetRelativeScale3D` (`self.FirstChain`) (0.0 0.0 0.0))
      (`SceneComponent.K2_SetRelativeLocationAndRotation` :`self` (`self.Sphere`)))
    (:`NewEnumerator2`
      (`InstancedStaticMeshComponent.ClearInstances` (`self.InstancedChains`))
      (set `self.CurrentHookLocation` (`self.K2_GetActorLocation`)))
    (:`NewEnumerator5`
      (`self.HandleSetHookShotState` "NewEnumerator1"))))

(fn `UserConstructionScript`)