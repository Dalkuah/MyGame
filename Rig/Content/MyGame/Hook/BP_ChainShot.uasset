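; Hookshot chain actor owned by BP_PlayerOX that latches onto a selected target and damages it based on the owner's attack stat.
; A Tick-driven state machine moves the hook out, pins it to the moving target, then retracts on ChainDead, dealing damage each retracting frame.
; The chain draws as instanced segments plus a scaled remainder link.
; It destroys itself once retracted or when the target becomes invalid.
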(event `/Game/MyGame/Hook/ChainSelect.ChainSelect`
  (params (TargetSelect :type "Actor Object Reference"))
  (set `self.Target` TargetSelect)
  (set `self.TargetHookShotLocation` (`self.K2_GetActorLocation` TargetSelect))
  (`self.HandleSetHookShotState` "NewEnumerator2")
  (set `self.HitSuccessful` true))

(event `/Game/MyGame/Hook/ChainSelect.ChainDead`
  (params (DeadTarget :type "Actor Object Reference"))
  (`self.HandleSetHookShotState` "NewEnumerator3")
  (bind _asbp_player_ox (cast `/Game/aaaaa/ThirdPerson/Blueprints/BP_PlayerOX` (`self.GetOwner`)))
  (`KismetArrayLibrary.Array_RemoveItem` (`/Game/aaaaa/ThirdPerson/Blueprints/BP_PlayerOX.Chain` _asbp_player_ox) self)
  (set `/Game/aaaaa/ThirdPerson/Blueprints/BP_PlayerOX.SkillUse` false _asbp_player_ox))

(event `self.ReceiveBeginPlay`
  (`self.HandleSetHookShotState` "NewEnumerator1"))

(event `self.ReceiveTick`
  (params (DeltaSeconds :type "Float (single-precision)"))
  (bind _target (`self.Target`))
  (bind _target_2 (`self.Target`))
  (bind _target_3 (`self.Target`))
  (bind _target_4 (`self.Target`))
  (bind _currenthooklocation (`self.CurrentHookLocation`))
  (bind _returnvalue (`self.K2_GetActorLocation` _target_4))
  (bind _returnvalue_2 (`KismetMathLibrary.GetDirectionUnitVector` (`self.K2_GetActorLocation`) (`self.CurrentHookLocation`)))
  (bind _returnvalue_3 (`InstancedStaticMeshComponent.GetInstanceCount` (`self.InstancedChains`)))
  (bind (_remainder _returnvalue_4) (`KismetMathLibrary.FMod` (`KismetMathLibrary.Vector_Distance` (`self.K2_GetActorLocation`) (`self.CurrentHookLocation`)) (`self.ChainMeshLength`)))
  (`|ExecutionSequence`
    (:`then_0`
      (if (`|EnumInequality` (`self.HookShotState`) "NewEnumerator1")
        (`|ExecutionSequence`
          (:`then_0`
            ;[1 1 1] 코멘트
            (`SceneComponent.K2_SetWorldLocationAndRotation` (`self.Sphere`) _currenthooklocation (`KismetMathLibrary.Conv_VectorToRotator` (`KismetMathLibrary.GetDirectionUnitVector` (`self.K2_GetActorLocation`) _currenthooklocation)) false false))
          (:`then_1`
            ;[1 1 1] 코멘트
            (`SceneComponent.K2_SetWorldRotation` (`self.FirstChain`) (`KismetMathLibrary.Conv_VectorToRotator` (`KismetMathLibrary.GetDirectionUnitVector` (`self.K2_GetActorLocation`) (`self.CurrentHookLocation`))) false false)
            (`SceneComponent.SetRelativeScale3D` (`self.FirstChain`) (`KismetMathLibrary.MakeVector` (/ (`KismetMathLibrary.FMod` (`KismetMathLibrary.Vector_Distance` (`self.K2_GetActorLocation`) (`self.CurrentHookLocation`)) (`self.ChainMeshLength`)) (`self.ChainMeshLength`)) 1.0 1.0)))
          (:`then_2`
            ;[1 1 1] 코멘트
            (`SceneComponent.K2_SetWorldLocationAndRotation` (`self.InstancedChains`) (+ (`self.K2_GetActorLocation`) (* _returnvalue_2 (`KismetMathLibrary.FMod` (`KismetMathLibrary.Vector_Distance` (`self.K2_GetActorLocation`) (`self.CurrentHookLocation`)) (`self.ChainMeshLength`)))) (`KismetMathLibrary.Conv_VectorToRotator` _returnvalue_2) false false)
            (if (> _returnvalue_4 _returnvalue_3)
              (for _index (range _returnvalue_3 _returnvalue_4)
                (`InstancedStaticMeshComponent.AddInstance` (`self.InstancedChains`) (`KismetMathLibrary.MakeTransform` (`KismetMathLibrary.MakeVector` (* _index (`self.ChainMeshLength`)))) false))
              (elif (< _returnvalue_4 _returnvalue_3)
                (for _index_2 (range _returnvalue_4 _returnvalue_3)
                  (`InstancedStaticMeshComponent.RemoveInstance` (`self.InstancedChains`) _index_2))))))))
    (:`then_1`
      (switch `/Game/MyGame/Hook/EN_HookShotState` (`self.HookShotState`)
        (:`NewEnumerator2`
          (set `self.CurrentHookLocation` (`KismetMathLibrary.VInterpTo_Constant` (`self.CurrentHookLocation`) (`self.TargetHookShotLocation`) DeltaSeconds (`self.ChainSpeed`)))
          (if (== (`self.CurrentHookLocation`) (`self.TargetHookShotLocation`))
            (if (`self.HitSuccessful`)
              (`self.HandleSetHookShotState` "NewEnumerator4")
              (`/Engine/EditorBlueprintResources/StandardMacros.IsValid` _target_3
                (:`Is Valid`
                  (bind _asbp_player_ox (cast `/Game/aaaaa/ThirdPerson/Blueprints/BP_PlayerOX` (`self.GetOwner`)))
                  (message `/Game/MyGame/AI/AttackOK.OK!` _target_3 (make `/Game/MyGame/AI/ST_Attack` (* (`/Game/aaaaa/ThirdPerson/Blueprints/BP_PlayerOX.공격력` _asbp_player_ox) 0.01) _asbp_player_ox "사슬" _target_3))))
              (else
                (`self.HandleSetHookShotState` "NewEnumerator3")))))
        (:`NewEnumerator3`
          (set `self.CurrentHookLocation` (`KismetMathLibrary.VInterpTo_Constant` (`self.CurrentHookLocation`) (`self.K2_GetActorLocation`) DeltaSeconds (`self.ChainSpeed`)))
          (if (== (`self.CurrentHookLocation`) (`self.K2_GetActorLocation`))
            (`self.HandleSetHookShotState` "NewEnumerator1")
            (`self.K2_DestroyActor`)
            (else
              (`/Engine/EditorBlueprintResources/StandardMacros.IsValid` _target_2
                (:`Is Valid`
                  (bind _asbp_player_ox_2 (cast `/Game/aaaaa/ThirdPerson/Blueprints/BP_PlayerOX` (`self.GetOwner`)))
                  (message `/Game/MyGame/AI/AttackOK.OK!` _target_2 (make `/Game/MyGame/AI/ST_Attack` (* (`/Game/aaaaa/ThirdPerson/Blueprints/BP_PlayerOX.공격력` _asbp_player_ox_2) 5.0) _asbp_player_ox_2 "사슬" _target_2)))))))))
    (:`then_2`
      (`/Engine/EditorBlueprintResources/StandardMacros.IsValid` _target_4
        (:`Is Valid`
          (set `self.HitSuccessful` true)
          (set `self.TargetHookShotLocation` _returnvalue))))
    (:`then_3`
      (`/Engine/EditorBlueprintResources/StandardMacros.IsValid` _target_4
        (:`Is Valid`
          (if (`|EnumEquality` (`self.HookShotState`) "NewEnumerator4")
            (set `self.CurrentHookLocation` _returnvalue)))
        (:`Is Not Valid`
          (`self.K2_DestroyActor`))))
    (:`then_4`
      (`/Engine/EditorBlueprintResources/StandardMacros.IsValid` _target
        (:`Is Valid`
          (message `/Game/MyGame/Hook/ChainSelect.ChainDead?` _target _target self))))))

(fn `CalculateHookShotHit`
  (params (CharacterCamera :type "CameraComponent Object Reference") (Target :type "Actor Object Reference"))
  (returns (EndCharacterLcoation :type "Vector Structure") (HitSuccessful :type Boolean))
  (bind _output_get (set `self.TargetHookShotLocation` (`self.K2_GetActorLocation` Target)))
  (`self.HandleSetHookShotState` "NewEnumerator2")
  (set `self.HitSuccessful` true)
  (return _output_get true))

(fn `HandleSetHookShotState`
  (params (NewHookShotState :type "/Game/MyGame/Hook/EN_HookShotState Enum" :default "NewEnumerator0"))
  (bind _output_get (set `self.HookShotState` NewHookShotState))
  (`self.OnHookShotStateChanged` _output_get)
  (switch `/Game/MyGame/Hook/EN_HookShotState` _output_get
    (:`NewEnumerator1`
      (`InstancedStaticMeshComponent.ClearInstances` (`self.InstancedChains`))
      (`SceneComponent.SetRelativeScale3D` (`self.FirstChain`) (0.0 0.0 0.0))
      (`SceneComponent.K2_SetRelativeLocationAndRotation` :`self` (`self.Sphere`)))
    (:`NewEnumerator2`
      (`InstancedStaticMeshComponent.ClearInstances` (`self.InstancedChains`))
      (set `self.CurrentHookLocation` (`self.K2_GetActorLocation`)))
    (:`NewEnumerator5`
      (`self.HandleSetHookShotState` "NewEnumerator1"))))

(fn `UserConstructionScript`)