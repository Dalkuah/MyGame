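; BP_Damage is a short-lived floating damage number that pops upward and disappears.
; On BeginPlay it launches its Box with an upward physics impulse, then destroys itself after a brief delay.
; The DamageText event shows the rounded-down damage on the Damage text component, and Crit recolors that text.
; Tick billboards the text by rotating it toward the player camera every frame.
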(event `self.ReceiveBeginPlay`
  (`PrimitiveComponent.AddImpulse` (`self.Box`) (0.0 0.0 500.0) "None" false)
  (`KismetSystemLibrary.Delay` 2.0)
  (`self.K2_DestroyActor`))

(event `Crit`
  (`TextRenderComponent.SetTextRenderColor` (`self.Damage`) (`self.Value`)))

(event `self.ReceiveTick`
  (params (DeltaSeconds :type "Float (single-precision)"))
  (bind _damage (`self.Damage`))
  (`SceneComponent.K2_SetWorldRotation` _damage (`KismetMathLibrary.FindLookAtRotation` (`SceneComponent.K2_GetComponentLocation` _damage) (`self.K2_GetActorLocation` (`GameplayStatics.GetPlayerCameraManager` 0))) false false))

(event `DamageText`
  (params (Damage :type "Float (double-precision)"))
  (`TextRenderComponent.K2_SetText` (`self.Damage`) (`KismetTextLibrary.Conv_StringToText` (`KismetStringLibrary.Conv_IntToString` (`KismetMathLibrary.FFloor` Damage)))))

(fn `UserConstructionScript`)